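; Player controller that tracks the collectible tools and relays game progress to the HUD.
; On BeginPlay it caches BP_HUD, then each ToolCollected event marks that tool's flag in a bool array, plays a sound and updates the HUD.
; When no false flag remains, it updates the objective and notifies BP_ThirdPersonGameMode.
; Timer updates, the game over screen and high score saving are pass-through calls to the HUD.
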(event `self.ReceiveBeginPlay`
  (bind _asbp_hud (cast `/Game/CustomBlueprints/HUD/BP_HUD` (`self.GetHUD`)))
  (set `self.HUDRef` _asbp_hud))

(event `ToolCollected`
  (params (ToolID :type Integer))
  (`KismetArrayLibrary.Array_Set` (`self.toolsToCollectArray`) ToolID true)
  (`GameplayStatics.PlaySound2D` "/Game/CustomBlueprints/Sounds/ActionSounds/ToolCollectedSound.ToolCollectedSound" 0.2 1.0 0.0 null null)
  (`/Game/CustomBlueprints/HUD/BP_HUD.UpdateItemsToCollectOnHUD` (`self.HUDRef`) ToolID)
  (if (not (`KismetArrayLibrary.Array_Contains` (`self.toolsToCollectArray`)))
    (`/Game/CustomBlueprints/HUD/BP_HUD.UpdateObjectiveOnHUD` (`self.HUDRef`))
    (bind _asbp_third_person_game_mode (cast `/Game/ThirdPerson/Blueprints/BP_ThirdPersonGameMode` (`GameplayStatics.GetGameMode`)))
    (`/Game/ThirdPerson/Blueprints/BP_ThirdPersonGameMode.LastCollectableCollected` _asbp_third_person_game_mode)))

(event `/Game/CustomBlueprints/Controller/BPI_Controller.SaveGame`
  (params (highScore :type "Float (double-precision)"))
  (`/Game/CustomBlueprints/HUD/BP_HUD.SaveHighScore` (`self.HUDRef`) highScore))

(fn `ShowGameOverScreen`
  (params (ScoreInTime :type "Float (double-precision)"))
  (`/Game/CustomBlueprints/HUD/BP_HUD.ShowGameOverScreen` (`self.HUDRef`) ScoreInTime))

(fn `UpdateTimerOnHUD`
  (params (time :type "Float (double-precision)"))
  (`/Game/CustomBlueprints/HUD/BP_HUD.UpdateTimerOnHud` (`self.HUDRef`) time))

(fn `UserConstructionScript`)