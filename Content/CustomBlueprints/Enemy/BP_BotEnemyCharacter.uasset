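; BP_BotEnemyCharacter is a wandering enemy bot that sets off an alarm and costs the player a time penalty on contact.
; A looping timer started on BeginPlay periodically sends it via AIMoveTo to a random navigable point within RandomMovementRadius of its current location.
; When its capsule overlaps the player pawn, it plays a 2D alarm sound and calls AddPenalityToTime on the cached BP_ThirdPersonGameMode.
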(event `self.ReceiveBeginPlay`
  (`|ExecutionSequence`
    (:`then_0`
      (bind _asbp_third_person_game_mode (cast `/Game/ThirdPerson/Blueprints/BP_ThirdPersonGameMode` (`GameplayStatics.GetGameMode`)))
      (set `self.GamemodeRef` _asbp_third_person_game_mode))
    (:`then_1`
      (`KismetSystemLibrary.K2_SetTimerDelegate` (delegate `ChoosePositionToMoveTo`) 5.0 true))))

(event `ChoosePositionToMoveTo`
  (bind _randomlocation (`NavigationSystemV1.K2_GetRandomLocationInNavigableRadius` (`SceneComponent.K2_GetComponentLocation` (`self.CapsuleComponent`)) (`self.randomMovementRadius`) null null))
  (`|AIMoveTo` self _randomlocation null))

(event `self.Capsule.OnComponentBeginOverlap`
  (params (OverlappedComponent :type "PrimitiveComponent Object Reference") (OtherActor :type "Actor Object Reference") (OtherComp :type "PrimitiveComponent Object Reference") (OtherBodyIndex :type Integer) (bFromSweep :type Boolean) (SweepResult :type "HitResult Structure (by ref)"))
  (if (== OtherActor (`GameplayStatics.GetPlayerPawn` 0))
    (`GameplayStatics.PlaySound2D` "/Game/CustomBlueprints/Sounds/ActionSounds/AlarmSound.AlarmSound" 0.5 1.0 0.0 null null)
    (`/Game/ThirdPerson/Blueprints/BP_ThirdPersonGameMode.AddPenalityToTime` (`self.GamemodeRef`))))

(fn `UserConstructionScript`)