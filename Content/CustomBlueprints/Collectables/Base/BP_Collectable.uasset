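; Base collectable tool pickup that takes its mesh from a table by tool ID and starts at a random yaw.
; A sphere overlap shows or hides the pickup widget for the player pawn, while a looping timer, rather than Tick, yaws the widget toward the player.
; CollectTool guards against repeat collection, then reports the tool ID to BP_Controller and destroys the actor.
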(event `self.ReceiveBeginPlay`
  (bind (_returnvalue_roll _returnvalue_pitch _returnvalue_yaw) (`KismetMathLibrary.BreakRotator` (`KismetMathLibrary.RandomRotator` false)))
  (`|ExecutionSequence`
    (:`then_0`
      (bind _asbp_third_person_character (cast `/Game/CustomBlueprints/Pawn/BP_ThirdPersonCharacter` (`GameplayStatics.GetPlayerPawn` 0)))
      (set `self.playerPawnRef` _asbp_third_person_character)
      (`SceneComponent.SetVisibility` (`self.PickUpWidget`) false false))
    (:`then_1`
      (`KismetSystemLibrary.K2_SetTimerDelegate` (delegate `RotateWidget`) 0.1 true)
      (`SceneComponent.K2_SetWorldRotation` (`self.ObjectToCollect`) (`KismetMathLibrary.MakeRotator` 0.0 0.0 _returnvalue_yaw) false false))))

(event `RotateWidget`
  (bind _pickupwidget (`self.PickUpWidget`))
  (bind (_returnvalue_roll _returnvalue_pitch _returnvalue_yaw) (`KismetMathLibrary.BreakRotator` (`KismetMathLibrary.FindLookAtRotation` (`SceneComponent.K2_GetComponentLocation` _pickupwidget) (`SceneComponent.K2_GetComponentLocation` (`Character.CapsuleComponent` (`self.playerPawnRef`))))))
  (`SceneComponent.K2_SetWorldRotation` _pickupwidget (`KismetMathLibrary.MakeRotator` 0.0 0.0 _returnvalue_yaw) false false))

(event `/Game/CustomBlueprints/Collectables/Base/BPI_SpawnTools.SpawnTool`
  (params (ToolID :type Integer))
  (bind _output_get (set `self.idOfTool` ToolID))
  (`StaticMeshComponent.SetStaticMesh` (`self.ObjectToCollect`) (`|GetArrayItem` (`self.toolMeshTable`) _output_get)))

(event `/Game/CustomBlueprints/Collectables/Base/BPI_Collectable.CollectTool`
  (if (not (`self.isCollected`))
    (set `self.isCollected` true)
    (`self.ToolCollected`)))

(event `ToolCollected`
  (bind _asbp_controller (cast `/Game/CustomBlueprints/Controller/BP_Controller` (`GameplayStatics.GetPlayerController` 0))
    (:`then`
      (`/Game/CustomBlueprints/Controller/BP_Controller.ToolCollected` _asbp_controller (`self.idOfTool`)))
    (:`CastFailed`
      _))
  (`self.K2_DestroyActor`))

(event `self.SphereCollision.OnComponentBeginOverlap`
  (params (OverlappedComponent :type "PrimitiveComponent Object Reference") (OtherActor :type "Actor Object Reference") (OtherComp :type "PrimitiveComponent Object Reference") (OtherBodyIndex :type Integer) (bFromSweep :type Boolean) (SweepResult :type "HitResult Structure (by ref)"))
  (if (== OtherActor (`self.playerPawnRef`))
    (`SceneComponent.SetVisibility` (`self.PickUpWidget`) true false)))

(event `self.SphereCollision.OnComponentEndOverlap`
  (params (OverlappedComponent :type "PrimitiveComponent Object Reference") (OtherActor :type "Actor Object Reference") (OtherComp :type "PrimitiveComponent Object Reference") (OtherBodyIndex :type Integer))
  (if (== OtherActor (`self.playerPawnRef`))
    (`SceneComponent.SetVisibility` (`self.PickUpWidget`) false false)))

(fn `UserConstructionScript`)