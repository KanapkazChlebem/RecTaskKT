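; Level exit door actor that ends the timed run when the player passes through it after it has opened.
; The Open event snaps the door part to its open transform, plays a sound and enables exiting.
; Once enabled, the player pawn overlapping the exit collision box triggers EndGame, which stops the timer on the cached BP_ThirdPersonGameMode.
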(event `self.ReceiveBeginPlay`
  (bind _asbp_third_person_game_mode (cast `/Game/ThirdPerson/Blueprints/BP_ThirdPersonGameMode` (`GameplayStatics.GetGameMode`)))
  (set `self.GamemodeRef` _asbp_third_person_game_mode))

(event `/Game/CustomBlueprints/Door/BPI_Exit.Open`
  (`SceneComponent.K2_SetRelativeTransform` (`self.SM_DoorPartToOpen`) (`self.OpenTransform`) false false)
  (set `self.CanExit` true)
  (`GameplayStatics.PlaySoundAtLocation` "/Game/CustomBlueprints/Sounds/ActionSounds/DoorOpening.DoorOpening" (`self.K2_GetActorLocation` self) (struct) 1.0 1.0 0.0 null null null null))

(event `self.CollisionBoxExit.OnComponentBeginOverlap`
  (params (OverlappedComponent :type "PrimitiveComponent Object Reference") (OtherActor :type "Actor Object Reference") (OtherComp :type "PrimitiveComponent Object Reference") (OtherBodyIndex :type Integer) (bFromSweep :type Boolean) (SweepResult :type "HitResult Structure (by ref)"))
  (if (`self.CanExit`)
    (if (== OtherActor (`GameplayStatics.GetPlayerPawn` 0))
      (`self.EndGame`))))

(event `EndGame`
  (`/Game/ThirdPerson/Blueprints/BP_ThirdPersonGameMode.StopTimer` (`self.GamemodeRef`)))

(fn `UserConstructionScript`)